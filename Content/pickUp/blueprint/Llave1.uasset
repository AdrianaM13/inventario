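; Key pickup actor that puts an item into the player's three-slot inventory on the TopDownCharacter.
; Any overlap with its Box destroys the Llave component, then writes item value 1 into the first empty slot among Espacio1 to Espacio3.
; The overlapping actor is not checked, and the Box stays active, so later overlaps can fill further slots.
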(event `self.Box.OnComponentBeginOverlap`
  (params (OverlappedComponent :type "PrimitiveComponent Object Reference") (OtherActor :type "Actor Object Reference") (OtherComp :type "PrimitiveComponent Object Reference") (OtherBodyIndex :type Integer) (bFromSweep :type Boolean) (SweepResult :type "HitResult Structure (by ref)"))
  (`ActorComponent.K2_DestroyComponent` (`self.llave`))
  (bind _astop_down_character (cast `/Game/TopDownBP/Blueprints/TopDownCharacter` (`GameplayStatics.GetPlayerCharacter` 0)))
  (if (== (`/Game/TopDownBP/Blueprints/TopDownCharacter.Espacio1` _astop_down_character) 0)
    (set `/Game/TopDownBP/Blueprints/TopDownCharacter.Espacio1` 1 _astop_down_character)
    (elif (== (`/Game/TopDownBP/Blueprints/TopDownCharacter.Espacio2` _astop_down_character) 0)
      (set `/Game/TopDownBP/Blueprints/TopDownCharacter.Espacio2` 1 _astop_down_character)
      (elif (== (`/Game/TopDownBP/Blueprints/TopDownCharacter.Espacio3` _astop_down_character) 0)
        (set `/Game/TopDownBP/Blueprints/TopDownCharacter.Espacio3` 1 _astop_down_character)))))

(fn `UserConstructionScript`)